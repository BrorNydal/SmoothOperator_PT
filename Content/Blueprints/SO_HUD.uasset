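; SO_HUD is a HUD Blueprint that shows the main menu, gameplay and death widgets.
; BeginPlay checks the level name, showing the menu with a mouse cursor in MainMenu, or blur and game widgets elsewhere.
; Tick polls the pawn's Dead flag, adding a new death widget and showing the cursor each frame it is true.
; The toddler check runs only after a successful bear cast finds Dead false.
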(event `self.ReceiveBeginPlay`
  (bind _returnvalue (`GameplayStatics.GetCurrentLevelName` true))
  (if (`KismetStringLibrary.EqualEqual_StrStr` _returnvalue "MainMenu")
    (bind _returnvalue_2 (`|CreateWidget` "/Game/Blueprints/bpMainMenuWidget.bpMainMenuWidget_C"))
    (`UserWidget.AddToViewport` _returnvalue_2 0)
    (set `PlayerController.bShowMouseCursor` true (`GameplayStatics.GetPlayerController` 0))
    (else
      (bind _returnvalue_3 (`|CreateWidget` "/Game/Blueprints/Blur.Blur_C"))
      (`UserWidget.AddToViewport` _returnvalue_3 0)
      (bind _returnvalue_4 (`|CreateWidget` "/Game/Blueprints/bpGameWidget.bpGameWidget_C"))
      (`UserWidget.AddToViewport` _returnvalue_4 0))))

(event `self.ReceiveTick`
  (params (DeltaSeconds :type "Float (single-precision)"))
  (bind _asbp_bear_character (cast `/Game/Blueprints/Characters/Bear/bpBearCharacter` (`GameplayStatics.GetPlayerPawn` 0)))
  (if (`BearCharacter.Dead` _asbp_bear_character)
    (bind _returnvalue (`|CreateWidget` "/Game/Blueprints/bpDead.bpDead_C" :!label _label))
    (`UserWidget.AddToViewport` _returnvalue 0)
    (set `PlayerController.bShowMouseCursor` true (`GameplayStatics.GetPlayerController` 0))
    (else
      (bind _asbp_toddler_character (cast `/Game/Blueprints/Characters/Toddler/bpToddlerCharacter` (`GameplayStatics.GetPlayerPawn` 0)))
      (if (`ToddlerCharacter.Dead` _asbp_toddler_character)
        (goto _label)))))

(fn `UserConstructionScript`)