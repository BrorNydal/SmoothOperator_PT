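; Playable toddler character that moves on world axes and can be launched by the bear character.
; Forward and right input add movement only while the toddler is not hidden.
; While airborne, Tick turns it to face its velocity.
; If the first bear found via GetAllActorsOfClass is launching, Tick also pushes the airborne toddler along that bear's forward vector with heavily scaled movement input.
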(event `InputAxis|MoveRight`
  (params (AxisValue :type "Float (single-precision)"))
  ;[1 1 1] Movement
  (if (not (`self.bHidden`))
    (`self.AddMovementInput` (0.0 1.0 0.0) AxisValue)))

(event `InputAxis|MoveForward`
  (params (AxisValue :type "Float (single-precision)"))
  ;[1 1 1] Movement
  (if (not (`self.bHidden`))
    (`self.AddMovementInput` (1.0 0.0 0.0) AxisValue)))

(event `self.ReceiveTick`
  (params (DeltaSeconds :type "Float (single-precision)"))
  (bind _returnvalue (`self.K2_GetActorLocation`))
  ;[1 1 1] Moving Forward When Launched/Not On The Ground
  (if (not (`NavMovementComponent.IsMovingOnGround` (`self.CharacterMovement`)))
    (`self.K2_SetActorRotation` (`KismetMathLibrary.FindLookAtRotation` _returnvalue (+ _returnvalue (`self.GetVelocity`))))
    (bind _outactors (`GameplayStatics.GetAllActorsOfClass` "/Game/Blueprints/bpBearCharacter.bpBearCharacter_C"))
    (bind _output (`|GetArrayItem` _outactors))
    (if (`/Game/Blueprints/bpBearCharacter.Launching` _output)
      (`self.AddMovementInput` (`self.GetActorForwardVector` _output) 2000.0))))

(fn `UserConstructionScript`)