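; AI-controlled enemy character that patrols between two waypoints and destroys the toddler character on contact.
; BeginPlay lowers walk speed and calls Patrol, which chains AIMoveTo to the first waypoint, a short delay, then AIMoveTo to the second.
; The patrol has no loop of its own: it restarts only when Hit reports a non-toddler actor.
; An unfinished array-based waypoint loop is left disconnected.
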(event `self.ReceiveBeginPlay`
  ;[1 1 1] Optional clamp (600 standard walk speed)
  (set `CharacterMovementComponent.MaxWalkSpeed` 300.0 (`self.CharacterMovement`))
  (`self.Patrol`))

(event `Patrol`
  ;[1 1 1] Makes the AI patrol between target point
  (`|AIMoveTo` self (0.0 0.0 0.0) (`self.Waypoint_0`)
    (:`OnSuccess`
      (`KismetSystemLibrary.Delay` 2.0)
      (`|AIMoveTo` self (0.0 0.0 0.0) (`self.Waypoint_1`)))))

(event `self.ReceiveHit`
  (params (MyComp :type "PrimitiveComponent Object Reference") (Other :type "Actor Object Reference") (OtherComp :type "PrimitiveComponent Object Reference") (bSelfMoved :type Boolean) (HitLocation :type "Vector Structure") (HitNormal :type "Vector Structure") (NormalImpulse :type "Vector Structure") (Hit :type "HitResult Structure (by ref)"))
  ;[1 1 1] If this enemy collides with the toddler, toddler gets destroyed! Note: getting a few camera errors in the ue4 log after actor is destroyed)
  (bind _astoddler_character (cast `ToddlerCharacter` Other)
    (:`then`
      (`self.K2_DestroyActor` _astoddler_character))
    (:`CastFailed`
      (`self.Patrol`))))

(fn `UserConstructionScript`)