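; Bear character with world-axis movement that visually shows whether the toddler is riding it.
; After a short BeginPlay delay, it copies the first toddler character's skeletal mesh onto BearSocketMesh and TutorialTPP.
; Each tick it toggles TutorialTPP visibility from IsRiding.
; Tick also keeps BearSocketMesh hidden, re-attaches it by the MyBackRide socket name and moves it to that socket on TutorialTPP, using the actor's rotation.
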(event `InputAxis|MoveRight`
  (params (AxisValue :type "Float (single-precision)"))
  ;[1 1 1] Movement
  (`self.AddMovementInput` (0.0 1.0 0.0) AxisValue))

(event `InputAxis|MoveForward`
  (params (AxisValue :type "Float (single-precision)"))
  ;[1 1 1] Movement
  (`self.AddMovementInput` (1.0 0.0 0.0) AxisValue))

(event `self.ReceiveTick`
  (params (DeltaSeconds :type "Float (single-precision)"))
  (bind _bearsocketmesh (`self.BearSocketMesh`))
  ;[1 1 1] Tick : Set visually if toddler is riding or not
  (`SceneComponent.SetHiddenInGame` _bearsocketmesh true false)
  (`SceneComponent.K2_AttachToComponent` _bearsocketmesh null "MyBackRide" "SnapToTarget" "SnapToTarget" "SnapToTarget" true)
  (`SceneComponent.K2_SetWorldLocationAndRotation` _bearsocketmesh (`SceneComponent.GetSocketLocation` (`self.TutorialTPP`) "MyBackRide") (`self.K2_GetActorRotation`) false false)
  (if (`self.IsRiding`)
    (`SceneComponent.SetHiddenInGame` (`self.TutorialTPP`) false false)
    (else
      (`SceneComponent.SetHiddenInGame` (`self.TutorialTPP`) true false))))

(event `self.ReceiveBeginPlay`
  ;[1 1 1] Begin_Play : Set TutorialTPP Mesh
  (`KismetSystemLibrary.Delay` 0.2)
  (bind _outactors (`GameplayStatics.GetAllActorsOfClass` "/Game/Blueprints/bpToddlerCharacter.bpToddlerCharacter_C"))
  (`SkinnedMeshComponent.SetSkinnedAssetAndUpdate` (`self.BearSocketMesh`) (`SkinnedMeshComponent.SkeletalMesh` (`Character.Mesh` (`|GetArrayItem` _outactors))) true)
  (`SkinnedMeshComponent.SetSkinnedAssetAndUpdate` (`self.TutorialTPP`) (`SkinnedMeshComponent.SkeletalMesh` (`self.BearSocketMesh`)) true))

(fn `UserConstructionScript`)