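; Enemy AI pawn that roams random navigable points, chases the toddler, and hides the toddler or bear on hit to "kill" them.
; PawnSensing sight or noise starts a timed chase toward the toddler, or resumes roaming if it is hidden.
; Tick triggers roaming when not attacking.
; Leaving a bpEnemyStop overlap clears InPosition, sending the pawn back toward the stop actor it overlapped at BeginPlay, confining its range.
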(event `self.ReceiveHit`
  (params (MyComp :type "PrimitiveComponent Object Reference") (Other :type "Actor Object Reference") (OtherComp :type "PrimitiveComponent Object Reference") (bSelfMoved :type Boolean) (HitLocation :type "Vector Structure") (HitNormal :type "Vector Structure") (NormalImpulse :type "Vector Structure") (Hit :type "HitResult Structure (by ref)"))
  ;[1 1 1] When hitting actors, kill them
  (bind _outactors (`GameplayStatics.GetAllActorsOfClass` "/Game/Blueprints/bpToddlerCharacter.bpToddlerCharacter_C"))
  (bind _output (`|GetArrayItem` _outactors))
  (if (== Other _output)
    (`self.SetActorHiddenInGame` _output true)
    (else
      (bind _outactors_2 (`GameplayStatics.GetAllActorsOfClass` "/Game/Blueprints/bpBearCharacter.bpBearCharacter_C"))
      (bind _output_2 (`|GetArrayItem` _outactors_2))
      (if (== _output_2 Other)
        (`self.SetActorHiddenInGame` _output_2 true)))))

(event `Roam`
  ;[1 1 1] Roam-Function
  (`|AIMoveTo` self (`NavigationSystemV1.K2_GetRandomLocationInNavigableRadius` (`self.K2_GetActorLocation`) 500.0 null null) null
    (:`OnSuccess`
      (`KismetSystemLibrary.Delay` 1.0)
      (`self.Roam`))))

(event `self.ReceiveBeginPlay`
  ;[1 1 1] Roam-Function
  (set `self.EnemyStop` (`|GetArrayItem` (`self.GetOverlappingActors` "/Game/Blueprints/bpEnemyStop.bpEnemyStop_C"))))

(event `self.PawnSensing.OnSeePawn`
  (params (Pawn :type "Pawn Object Reference"))
  ;[1 1 1] Pawn sense Toddler, goes to Location
  (bind _outactors (`GameplayStatics.GetAllActorsOfClass` "/Game/Blueprints/bpToddlerCharacter.bpToddlerCharacter_C" :!label _label))
  (bind _output (`|GetArrayItem` _outactors))
  (if (`Actor.bHidden` _output)
    (`self.Roam`)
    (else
      (set `self.Attacking` true)
      (if (`self.InPosition`)
        (`|AIMoveTo` self (`self.K2_GetActorLocation` _output) _output
          (:`then`
            (`KismetSystemLibrary.Delay` 7.0)
            (set `self.Attacking` false)))
        (else
          (`|AIMoveTo` self (`self.K2_GetActorLocation` (`self.EnemyStop`)) null
            (:`then`
              (`KismetSystemLibrary.Delay` 1.0)
              (set `self.InPosition` true)
              (set `self.Attacking` false))))))))

(event `self.PawnSensing.OnHearNoise`
  (params (Instigator :type "Pawn Object Reference") (Location :type "Vector Structure (by ref)") (Volume :type "Float (single-precision)"))
  ;[1 1 1] Pawn sense Toddler, goes to Location
  (goto _label))

(event `self.ReceiveTick`
  (params (DeltaSeconds :type "Float (single-precision)"))
  ;[1 1 1] Roam, when not attacking
  (if (`self.InPosition`)
    (if (not (`self.Attacking`))
      (`KismetSystemLibrary.Delay` 0.5)
      (`self.Roam`))
    (else
      (`|AIMoveTo` self (`self.K2_GetActorLocation` (`self.EnemyStop`)) null
        (:`then`
          (`KismetSystemLibrary.Delay` 1.0)
          (set `self.InPosition` true))))))

(event `self.ReceiveActorEndOverlap`
  (params (OtherActor :type "Actor Object Reference"))
  ;[1 1 1] Communicates with "bpEnemyStop" which tells this actor where it can't go
  (cast `/Game/Blueprints/bpEnemyStop` OtherActor)
  (set `self.InPosition` false))

(fn `UserConstructionScript`)