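; Tutorial trigger volume that tells the toddler or bear character which tutorial image to show.
; On box overlap begin, it writes its TutorialImage into the overlapping character's TutorialShowing variable; on overlap end, it clears that variable.
; Other actors are ignored, and the ShowTutorial function is empty.
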(event `self.Box.OnComponentBeginOverlap`
  (params (OverlappedComponent :type "PrimitiveComponent Object Reference") (OtherActor :type "Actor Object Reference") (OtherComp :type "PrimitiveComponent Object Reference") (OtherBodyIndex :type Integer) (bFromSweep :type Boolean) (SweepResult :type "HitResult Structure (by ref)"))
  (bind _asbp_toddler_character (cast `/Game/Blueprints/Characters/Toddler/bpToddlerCharacter` OtherActor)
    (:`then`
      (set `/Game/Blueprints/Characters/Toddler/bpToddlerCharacter.TutorialShowing` (`self.TutorialImage`) _asbp_toddler_character))
    (:`CastFailed`
      (bind _asbp_bear_character (cast `/Game/Blueprints/Characters/Bear/bpBearCharacter` OtherActor))
      (set `/Game/Blueprints/Characters/Bear/bpBearCharacter.TutorialShowing` (`self.TutorialImage`) _asbp_bear_character))))

(event `self.Box.OnComponentEndOverlap`
  (params (OverlappedComponent :type "PrimitiveComponent Object Reference") (OtherActor :type "Actor Object Reference") (OtherComp :type "PrimitiveComponent Object Reference") (OtherBodyIndex :type Integer))
  (bind _asbp_toddler_character (cast `/Game/Blueprints/Characters/Toddler/bpToddlerCharacter` OtherActor)
    (:`then`
      (set `/Game/Blueprints/Characters/Toddler/bpToddlerCharacter.TutorialShowing` (struct) _asbp_toddler_character))
    (:`CastFailed`
      (bind _asbp_bear_character (cast `/Game/Blueprints/Characters/Bear/bpBearCharacter` OtherActor))
      (set `/Game/Blueprints/Characters/Bear/bpBearCharacter.TutorialShowing` (struct) _asbp_bear_character))))

(fn `ShowTutorial`)

(fn `UserConstructionScript`)