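; SO_HUD creates the game's screen widgets, choosing between main menu and gameplay UI by the current level name.
; On BeginPlay, MainMenu gets the menu widget and mouse cursor, while other levels get Blur and game widgets.
; Outside the menu, Tick looks up the toddler and bear characters and, if either is Dead, adds the death widget and shows the cursor.
; That check has no guard, so it adds a new death widget every frame.
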(event `self.ReceiveBeginPlay`
  (bind _returnvalue (`GameplayStatics.GetCurrentLevelName` true))
  (if (`KismetStringLibrary.EqualEqual_StrStr` _returnvalue "MainMenu")
    (bind _returnvalue_2 (`|CreateWidget` "/Game/Blueprints/HUD_and_Widgets/bpMainMenuWidget.bpMainMenuWidget_C"))
    (`UserWidget.AddToViewport` _returnvalue_2 0)
    (set `PlayerController.bShowMouseCursor` true (`GameplayStatics.GetPlayerController` 0))
    (else
      (bind _returnvalue_3 (`|CreateWidget` "/Game/Blueprints/HUD_and_Widgets/Blur.Blur_C"))
      (`UserWidget.AddToViewport` _returnvalue_3 0)
      (bind _returnvalue_4 (`|CreateWidget` "/Game/Blueprints/HUD_and_Widgets/bpGameWidget.bpGameWidget_C"))
      (`UserWidget.AddToViewport` _returnvalue_4 0))))

(event `self.ReceiveTick`
  (params (DeltaSeconds :type "Float (single-precision)"))
  (bind _returnvalue (`GameplayStatics.GetCurrentLevelName` true))
  (if (not (`KismetStringLibrary.EqualEqual_StrStr` _returnvalue "MainMenu"))
    (bind _outactors (`GameplayStatics.GetAllActorsOfClass` "/Game/Blueprints/Characters/Toddler/bpToddlerCharacter.bpToddlerCharacter_C"))
    (bind _outactors_2 (`GameplayStatics.GetAllActorsOfClass` "/Game/Blueprints/Characters/Bear/bpBearCharacter.bpBearCharacter_C"))
    (if (or (`BearCharacter.Dead` (`|GetArrayItem` _outactors_2)) (`ToddlerCharacter.Dead` (`|GetArrayItem` _outactors)))
      (bind _returnvalue_2 (`|CreateWidget` "/Game/Blueprints/HUD_and_Widgets/bpDead.bpDead_C"))
      (`UserWidget.AddToViewport` _returnvalue_2 0)
      (set `PlayerController.bShowMouseCursor` true (`GameplayStatics.GetPlayerController` 0)))))

(fn `UserConstructionScript`)