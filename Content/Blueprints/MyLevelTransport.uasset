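; MyLevelTransport is a level exit that sends the player to the next map on overlap.
; The destination follows a hardcoded chain keyed on the current level name: TutorialLevel to Level1_Map, then Level1_Map to Level_2_Map.
; The construction script fills a text label from ObjectName, and Tick shows it only while the player is within a fixed distance.
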(event `self.ReceiveActorBeginOverlap`
  (params (OtherActor :type "Actor Object Reference"))
  (if (== OtherActor (`GameplayStatics.GetPlayerCharacter` 0))
    (bind _returnvalue (`GameplayStatics.GetCurrentLevelName` true))
    (if (`KismetStringLibrary.EqualEqual_StrStr` _returnvalue "TutorialLevel")
      (`GameplayStatics.OpenLevel` "Level1_Map")
      (elif (`KismetStringLibrary.EqualEqual_StrStr` _returnvalue "Level1_Map")
        (`GameplayStatics.OpenLevel` "Level_2_Map")))))

(event `self.ReceiveTick`
  (params (DeltaSeconds :type "Float (single-precision)"))
  (bind _textrender (`self.TextRender`))
  (if (<= (`KismetMathLibrary.VSize` (- (`self.K2_GetActorLocation` (`GameplayStatics.GetPlayerCharacter` 0)) (`self.K2_GetActorLocation`))) 1000.0)
    (`SceneComponent.SetVisibility` _textrender true false)
    (else
      (`SceneComponent.SetVisibility` _textrender false false))))

(fn `UserConstructionScript`
  (`TextRenderComponent.K2_SetText` (`self.TextRender`) (`self.ObjectName`)))